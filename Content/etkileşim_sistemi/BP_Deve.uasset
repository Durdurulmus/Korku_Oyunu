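; Elevator Blueprint that moves a lift between top and bottom positions, triggered by a box overlap after a short delay or by the E key.
; Two switch colliders show a call prompt widget and enable input for overlapping player actors, undoing both on exit.
; ActivateSwitches uses IsAtBottom to set red/green light materials and enable only one switch collider.
; MoveComponentTo scales travel time with distance for constant speed, and IsAtBottom flips with each move.
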(event OnComponentBeginOverlap(SwitchCollider)
  (params (OverlappedComponent :type Primitive%20Component%20Object%20Reference) (OtherActor :type Actor%20Object%20Reference) (OtherComp :type Primitive%20Component%20Object%20Reference) (OtherBodyIndex :type Integer) (bFromSweep :type Boolean) (SweepResult :type Hit%20Result%20Structure%20%28by%20ref%29))
  (Utilities|CheckandEnableInput OtherActor))

(event OnComponentBeginOverlap(Box)
  (params (OverlappedComponent :type Primitive%20Component%20Object%20Reference) (OtherActor :type Actor%20Object%20Reference) (OtherComp :type Primitive%20Component%20Object%20Reference) (OtherBodyIndex :type Integer) (bFromSweep :type Boolean) (SweepResult :type Hit%20Result%20Structure%20%28by%20ref%29))
  (Utilities|FlowControl|Delay 1.0)
  (CallFunction|MoveElevator))

(event OnComponentBeginOverlap(SwitchCollider1)
  (params (OverlappedComponent :type Primitive%20Component%20Object%20Reference) (OtherActor :type Actor%20Object%20Reference) (OtherComp :type Primitive%20Component%20Object%20Reference) (OtherBodyIndex :type Integer) (bFromSweep :type Boolean) (SweepResult :type Hit%20Result%20Structure%20%28by%20ref%29))
  (Utilities|CheckandEnableInput OtherActor))

(event OnComponentEndOverlap(SwitchCollider)
  (params (OverlappedComponent :type Primitive%20Component%20Object%20Reference) (OtherActor :type Actor%20Object%20Reference) (OtherComp :type Primitive%20Component%20Object%20Reference) (OtherBodyIndex :type Integer))
  (Utilities|CheckandDisableInput OtherActor))

(event OnComponentEndOverlap(SwitchCollider1)
  (params (OverlappedComponent :type Primitive%20Component%20Object%20Reference) (OtherActor :type Actor%20Object%20Reference) (OtherComp :type Primitive%20Component%20Object%20Reference) (OtherBodyIndex :type Integer))
  (Utilities|CheckandDisableInput OtherActor))

(event EventBeginPlay
  (CallFunction|ActivateSwitches (Variables|Default|GetIs%20at%20Bottom))
  (bind _returnvalue (UserInterface|CreateWidget "/Game/etkileşim_sistemi/UI/WDG_Instruction.WDG_Instruction_C" (Game|GetPlayerController 0)))
  (bind _output_get (Variables|Default|SetWDGInstruction _returnvalue))
  (Default|SetText _output_get "Call Evelator(E)"))

(event Input|KeyboardEvents|E
  (params (Key :type Key%20Structure :default "None"))
  (:Pressed
    (CallFunction|MoveElevator)
    (CallFunction|ActivateSwitches (not (Variables|Default|GetIs%20at%20Bottom)))))

(fn ConstructionScript)

(fn ActivateSwitches
  (params (Atbottom :type Boolean))
  (Rendering|Material|SetVectorParameterValueonMaterials (Variables|Default|GetStaticMesh2) "Lightcolor" (Math|Conversions|ToVector(LinearColor) (Math|Color|SelectColor "(R=1.000000,G=0.000000,B=0.030342,A=1.000000)" "(R=0.000000,G=1.000000,B=0.137440,A=1.000000)" Atbottom)))
  (Collision|SetCollisionEnabled (Variables|Default|GetSwitchCollider) (select Atbottom "NoCollision" "QueryAndPhysics"))
  (Rendering|Material|SetVectorParameterValueonMaterials (Variables|Default|GetStaticMesh4) "Lightcolor" (Math|Conversions|ToVector(LinearColor) (Math|Color|SelectColor "(R=1.000000,G=0.000000,B=0.030342,A=1.000000)" "(R=0.000000,G=1.000000,B=0.137440,A=1.000000)" (not Atbottom))))
  (Collision|SetCollisionEnabled (Variables|Default|GetSwitchCollider1) (select (not Atbottom) "NoCollision" "QueryAndPhysics")))

(event Custom|MoveElevator
  (bind _lift (Variables|Default|GetLift))
  (Components|MoveComponentTo _lift (Variables|/Script/Engine.SceneComponent|GetRelativeLocation (select (Variables|Default|GetIs%20at%20Bottom) (Variables|Default|GetLiftBottom) (Variables|Default|GetLiftTop))) "0, 0, 0" false false (/ (Math|Vector|Distance(Vector) (Variables|/Script/Engine.SceneComponent|GetRelativeLocation _lift) (Variables|/Script/Engine.SceneComponent|GetRelativeLocation (select (Variables|Default|GetIs%20at%20Bottom) (Variables|Default|GetLiftBottom) (Variables|Default|GetLiftTop)))) 1e+02) false)
  (Variables|Default|SetIs%20at%20Bottom (not (Variables|Default|GetIs%20at%20Bottom)))
  (return))
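; Skinwalker monster that roams the level, chases the player on sight and performs a jumpscare attack on contact.
; AIMoveTo drives a looping random navmesh wander, while PawnSensing redirects it toward the player and manages chase audio.
; A retriggerable delay returns it to roaming and fades the audio once sightings stop.
; A one-time capsule hit destroys the flashlight, blends the camera to the monster, plays the attack montage and shows a widget.
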(event OnSeePawn(PawnSensing)
  (params (Pawn :type Pawn%20Object%20Reference))
  (bind _returnvalue (Game|GetPlayerCharacter 0))
  ;[0.15 0.15 0.15 0.5] Comment
  (if (== Pawn _returnvalue)
    (Utilities|FlowControl|Sequence
      (:then_0
        (Variables|Default|Setseeplayer? false)
        (AI|AIMoveTo self "0, 0, 0" _returnvalue 5.0 false
          (:then
            (Variables|Default|GetChasesequence
              (:then)
              (:else
                (bind _returnvalue_2 (Audio|SpawnSound2D "/Game/etkileşim_sistemi/Monster/Sounds/chasesequence.chasesequence" 1.0 1.0 0.0 0))
                (bind _output_get (Variables|Default|SetChasesequence _returnvalue_2))
                (Audio|Components|Audio|FadeIn _output_get 1.0 1.0 0.0 "Linear" :!class /Script/Engine.AudioComponent))))))
      (:then_1
        (Utilities|FlowControl|RetriggerableDelay 1.5)
        (Variables|Default|Setseeplayer? false)
        (CallFunction|RandomIyroam)
        (bind _chasesequence (Variables|Default|GetChasesequence)
          (:then
            (Audio|Components|Audio|FadeOut _chasesequence 1.5 0.0 "Linear" :!class /Script/Engine.AudioComponent)
            (Utilities|FlowControl|Delay 1.0)
            (Variables|Default|SetChasesequence 0))
          (:else))))))

(event OnComponentHit(CapsuleComponent)
  (params (HitComponent :type Primitive%20Component%20Object%20Reference) (OtherActor :type Actor%20Object%20Reference) (OtherComp :type Primitive%20Component%20Object%20Reference) (NormalImpulse :type Vector :default "0, 0, 0") (Hit :type Hit%20Result%20Structure%20%28by%20ref%29))
  ;[0.15 0.15 0.15 0.5] Comment
  (bind _asmultiplayer_character (Utilities|Casting|CastToMultiplayerCharacter OtherActor))
  (Utilities|FlowControl|DoOnce false
    (:Completed
      (Actor|DestroyActor (Variables|/Game/etkileşim_sistemi/Blueprints/Framework/MultiplayerCharacter.MultiplayerCharacter_C|GetFlashlightref _asmultiplayer_character))
      (Game|Player|SetViewTargetwithBlend (Game|GetPlayerController 0) self 1.0 "VTBlend_Linear" 0.0 false)
      (bind _returnvalue (Animation|PlayAnimMontage "/Game/etkileşim_sistemi/Monster/Animation/monsterattack1_Montage.monsterattack1_Montage" 1.0 "None"))
      (Utilities|FlowControl|Delay (- _returnvalue 1.2))
      (bind _returnvalue_2 (UserInterface|CreateWidget 0))
      (UserInterface|Viewport|AddtoViewport _returnvalue_2 0))))

(event Custom|RandomIyroam
  ;[0.15 0.15 0.15 0.5] Comment
  (Development|PrintString "RandomIyroam")
  (Class|NavigationSystemV1|GetRandomLocationinNavigableRadius (Transformation|GetActorLocation) 0.0 0 0)
  (AI|AIMoveTo self "0, 0, 0" 0 5.0 false
    (:then
      (Utilities|FlowControl|Delay 4.0)
      (if (not (Variables|Default|Getseeplayer?))
        (CallFunction|RandomIyroam)))))

(event EventBeginPlay
  ;[0.15 0.15 0.15 0.5] Comment
  (Variables|/Script/Engine.CharacterMovementComponent|SetMaxWalkSpeed (Variables|Character|GetCharacterMovement) (Variables|Default|GetMonster%20speed))
  (Class|NavigationSystemV1|GetRandomLocationinNavigableRadius (Transformation|GetActorLocation) 0.0 0 0)
  (AI|AIMoveTo self "0, 0, 0" 0 5.0 false
    (:then
      (Utilities|FlowControl|Delay 4.0)
      (if (not (Variables|Default|Getseeplayer?))
        (CallFunction|RandomIyroam)))))

(fn ConstructionScript)